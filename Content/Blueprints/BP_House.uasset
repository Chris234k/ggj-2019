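; BP_House is a house actor that banks the player's power and food into the house inventory when the player enters.
; BeginPlay gathers BP_HouseInventory actors, and an EnterHouse overlap by a ThirdPersonCharacter passes the first one to TakeFromPlayer.
; TakeFromPlayer adds both player amounts, each clamped between zero and the house's total Capacity, without deducting them from the player's inventory in this graph.
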(event `self.ReceiveBeginPlay`
  (bind _outactors (`GameplayStatics.GetAllActorsOfClass` "/Game/Blueprints/BP_HouseInventory.BP_HouseInventory_C")))

(event `self.EnterHouse.OnComponentBeginOverlap`
  (params (OverlappedComponent :type "PrimitiveComponent Object Reference") (OtherActor :type "Actor Object Reference") (OtherComp :type "PrimitiveComponent Object Reference") (OtherBodyIndex :type Integer) (bFromSweep :type Boolean) (SweepResult :type "HitResult Structure (by ref)"))
  (bind _asthird_person_character (cast `/Game/ThirdPersonBP/Blueprints/ThirdPersonCharacter` OtherActor))
  (`self.TakeFromPlayer` (`/Game/ThirdPersonBP/Blueprints/ThirdPersonCharacter.Player_Inventory` _asthird_person_character) (`|GetArrayItem` (stale `self.ReceiveBeginPlay` _outactors))))

(fn `TakeFromPlayer`
  (params (PlayerInventory :type "/Game/Blueprints/Player_Inventory Object Reference") (HouseInventory :type "/Game/Blueprints/BP_HouseInventory Object Reference"))
  (bind _capacity (`/Game/Blueprints/BP_HouseInventory.Capacity` HouseInventory))
  (`/Game/Blueprints/BP_HouseInventory.AddResource` HouseInventory "NewEnumerator1" (`KismetMathLibrary.Clamp` (`/Game/Blueprints/Player_Inventory.CurrentPower` PlayerInventory) 0 _capacity))
  (`/Game/Blueprints/BP_HouseInventory.AddResource` HouseInventory "NewEnumerator2" (`KismetMathLibrary.Clamp` (`/Game/Blueprints/Player_Inventory.CurrentFood` PlayerInventory) 0 _capacity)))

(fn `UserConstructionScript`)