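; BPC_UnlockManager is a component that tracks which player and house upgrades are unlocked.
; On BeginPlay it fills two boolean arrays with false, one slot per value of the player unlock and house unlock enums.
; Getter and setter functions read or write each array by converting the enum value to an index, so the enum order defines the layout.
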(event `self.ReceiveBeginPlay`
  (foreach `/Game/Blueprints/EPlayerUnlocks` true
    (:`LoopBody`
      (`KismetArrayLibrary.Array_Add` (`self.PlayerUnlockedArray`)))
    (:`then`
      (foreach `/Game/Blueprints/EHouseUnlocks` true
        (:`LoopBody`
          (`KismetArrayLibrary.Array_Add` (`self.HouseUnlocksArray`)))))))

(fn `IsHoueUpgradeUnlocked`
  (params (HouseUpgradeType :type "/Game/Blueprints/EHouseUnlocks Enum" :default "NewEnumerator0"))
  (returns (IsUnlocked :type Boolean))
  (return (`|GetArrayItem` (`self.HouseUnlocksArray`) (`KismetMathLibrary.Conv_ByteToInt` HouseUpgradeType))))

(fn `IsPlayerUpgradeUnlocked`
  (params (UnlockType :type "/Game/Blueprints/EPlayerUnlocks Enum" :default "NewEnumerator0"))
  (returns (IsUnlocked :type Boolean))
  (return (`|GetArrayItem` (`self.PlayerUnlockedArray`) (`KismetMathLibrary.Conv_ByteToInt` UnlockType))))

(fn `SetHouseUpgradeUnlock`
  (params (isUnlocked :type Boolean) (PlayerUpgradeType :type "/Game/Blueprints/EPlayerUnlocks Enum" :default "NewEnumerator0"))
  (`KismetArrayLibrary.Array_Set` (`self.HouseUnlocksArray`) (`KismetMathLibrary.Conv_ByteToInt` PlayerUpgradeType) isUnlocked))

(fn `SetPlayerUpgradeUnlock`
  (params (isUnlocked :type Boolean) (PlayerUpgradeType :type "/Game/Blueprints/EPlayerUnlocks Enum" :default "NewEnumerator0"))
  (`KismetArrayLibrary.Array_Set` (`self.PlayerUnlockedArray`) (`KismetMathLibrary.Conv_ByteToInt` PlayerUpgradeType) isUnlocked))