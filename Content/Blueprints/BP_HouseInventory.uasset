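; House inventory Blueprint that tracks the player's Oxygen, Power, Food and Water and shows them in a WBP_Inventory widget created at BeginPlay.
; AddResource clamps gains to MaxCapacity, while ConsumeItem adds an item's values unclamped; number keys top up each resource.
; AttemptPurchase deducts a crafting button's costs if affordable, but its returned affordability reads the balances left after deduction.
; UpdateUI pushes the totals to the widget after changes.
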(event `Key|One`
  (params (Key :type "Key Structure"))
  (:`Pressed`
    (`self.AddResource` "NewEnumerator0" 100)
    (`self.UpdateUI`)))

(event `Key|Two`
  (params (Key :type "Key Structure"))
  (:`Pressed`
    (`self.AddResource` "NewEnumerator1" 100)
    (`self.UpdateUI`)))

(event `Key|Three`
  (params (Key :type "Key Structure"))
  (:`Pressed`
    (`self.AddResource` "NewEnumerator2" 100)
    (`self.UpdateUI`)))

(event `Key|Four`
  (params (Key :type "Key Structure"))
  (:`Pressed`
    (`self.AddResource` "NewEnumerator3" 100)
    (`self.UpdateUI`)))

(event `self.ReceiveBeginPlay`
  (bind _returnvalue (`|CreateWidget` "/Game/Blueprints/WBP_Inventory.WBP_Inventory_C"))
  (bind _output_get (set `self.UI` _returnvalue))
  (`UserWidget.AddToViewport` _output_get 0))

(fn `AddResource`
  (params (resource :type "/Game/Blueprints/EResourceType Enum" :default "NewEnumerator0") (amount :type Integer))
  (returns (total :type Integer))
  (switch `/Game/Blueprints/EResourceType` resource
    (:`NewEnumerator0`
      (bind _output_get (set `self.Oxygen` (`KismetMathLibrary.Clamp` (+ amount (`self.Oxygen`)) 0 (`self.MaxCapacity`))))
      (`self.UpdateUI`)
      (return _output_get))
    (:`NewEnumerator1`
      (bind _output_get_2 (set `self.Power` (`KismetMathLibrary.Clamp` (+ amount (`self.Power`)) 0 (`self.MaxCapacity`))))
      (`self.UpdateUI`)
      (return _output_get_2))
    (:`NewEnumerator2`
      (bind _output_get_3 (set `self.Food` (`KismetMathLibrary.Clamp` (+ amount (`self.Food`)) 0 (`self.MaxCapacity`))))
      (`self.UpdateUI`)
      (return _output_get_3))
    (:`NewEnumerator3`
      (bind _output_get_4 (set `self.Water` (`KismetMathLibrary.Clamp` (+ amount (`self.Water`)) 0 (`self.MaxCapacity`))))
      (`self.UpdateUI`)
      (return _output_get_4))))

(fn `AttemptPurchase`
  (params (CraftingButton :type "/Game/Blueprints/WBP_CraftingButton Object Reference"))
  (returns (Result :type Boolean))
  (bind _oxygen (`self.Oxygen`))
  (bind _water (`self.Water`))
  (bind _oxygencost (`/Game/Blueprints/WBP_CraftingButton.OxygenCost` CraftingButton))
  (bind _power (`self.Power`))
  (bind _food (`self.Food`))
  (bind _watercost (`/Game/Blueprints/WBP_CraftingButton.WaterCost` CraftingButton))
  (bind _foodcost (`/Game/Blueprints/WBP_CraftingButton.FoodCost` CraftingButton))
  (bind _powercost (`/Game/Blueprints/WBP_CraftingButton.PowerCost` CraftingButton))
  (bind _returnvalue (and (>= _oxygen _oxygencost) (>= _water _watercost) (>= _power _powercost) (>= _food _foodcost)))
  (if _returnvalue
    ;[1 1 1] Can Afford, make purchase
    (set `self.Oxygen` (- _oxygen _oxygencost))
    (set `self.Water` (- _water _watercost))
    (set `self.Power` (- _power _powercost))
    (set `self.Food` (- _food _foodcost))
    (`self.UpdateUI`))
  (return _returnvalue))

(fn `ConsumeItem`
  (params (item :type "/Game/Blueprints/BP_Item Object Reference"))
  ;[1 1 1] Oxygen
  (set `self.Oxygen` (+ (`/Game/Blueprints/BP_Item.Oxygen` item) (`self.Oxygen`)))
  ;[1 1 1] Power
  (set `self.Power` (+ (`/Game/Blueprints/BP_Item.Power` item) (`self.Power`)))
  ;[1 1 1] Water
  (set `self.Water` (+ (`/Game/Blueprints/BP_Item.Water` item) (`self.Water`)))
  ;[1 1 1] Food
  (set `self.Food` (+ (`/Game/Blueprints/BP_Item.Food` item) (`self.Food`)))
  (`self.UpdateUI`))

(fn `UpdateUI`
  (set `/Game/Blueprints/WBP_Inventory.Oxygen` (`self.Oxygen`) (`self.UI`))
  (set `/Game/Blueprints/WBP_Inventory.Power` (`self.Power`) (`self.UI`))
  (set `/Game/Blueprints/WBP_Inventory.Food` (`self.Food`) (`self.UI`))
  (set `/Game/Blueprints/WBP_Inventory.Water` (`self.Water`) (`self.UI`)))

(fn `UserConstructionScript`)