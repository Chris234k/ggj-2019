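; BP_OxygenGenerator is a generator that periodically adds a resource, presumably oxygen given its name, to the house inventory.
; BeginPlay caches the first BP_HouseInventory found in the level.
; Tick accumulates delta time until it exceeds GenerationCD, then resets the timer and calls AddResource on that inventory for one unit of the resource enum's NewEnumerator0 entry.
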(event `self.ReceiveBeginPlay`
  (bind _outactors (`GameplayStatics.GetAllActorsOfClass` "/Game/Blueprints/BP_HouseInventory.BP_HouseInventory_C"))
  (set `self.HouseInventory` (`|GetArrayItem` _outactors)))

(event `self.ReceiveTick`
  (params (DeltaSeconds :type "Float (single-precision)"))
  (bind _output_get (set `self.GenerationTimer` (+ DeltaSeconds (`self.GenerationTimer`))))
  (if (> _output_get (`self.GenerationCD`))
    (set `self.GenerationTimer` 0.0)
    (`/Game/Blueprints/BP_HouseInventory.AddResource` (`self.HouseInventory`) "NewEnumerator0" 1)))

(fn `UserConstructionScript`)