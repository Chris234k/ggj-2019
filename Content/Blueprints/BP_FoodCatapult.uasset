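; BP_FoodCatapult is a placeholder actor, marked by a TODO as a copy of BP_OxygenGenerator that still lacks food catapult functionality.
; BeginPlay caches the first BP_HouseInventory found in the level.
; A timer that would add one resource unit to that inventory each cooldown is left disconnected, so Tick does nothing and the actor produces nothing.
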(event `self.ReceiveBeginPlay`
  ;[1 1 1] TODO(chris) THIS IS 100% A COPY OF BP_OXYGENGENERATOR PLS ADD FOOD CATAPULT FUNCTIONALITY
  (bind _outactors (`GameplayStatics.GetAllActorsOfClass` "/Game/Blueprints/BP_HouseInventory.BP_HouseInventory_C"))
  (set `self.HouseInventory` (`|GetArrayItem` _outactors)))

(event `self.ReceiveTick`
  (params (DeltaSeconds :type "Float (single-precision)"))
  ;[1 1 1] TODO(chris) THIS IS 100% A COPY OF BP_OXYGENGENERATOR PLS ADD FOOD CATAPULT FUNCTIONALITY
)

(fn `UserConstructionScript`)