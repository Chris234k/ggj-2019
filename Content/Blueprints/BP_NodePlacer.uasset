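; BP_NodePlacer scatters resource nodes at random points inside its Box component when play begins.
; Each spawned BP_RescourceNode receives the placer's resource multiplier and amount plus a fixed spawn time.
; SpawnNewNode, uncalled here, attempts rejection sampling outside an inner box but re-rolls the point at spawn, then appends the node to an array.
; GenerateNodes and the construction script are empty.
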(event `self.ReceiveBeginPlay`
  (bind (_origin _boxextent) (`KismetSystemLibrary.GetComponentBounds` (`self.Box`)))
  (for _ (range 31)
    (bind _returnvalue (`|SpawnActorFromClass` "/Game/Blueprints/BP_RescourceNode.BP_RescourceNode_C" (`KismetMathLibrary.Conv_VectorToTransform` (`KismetMathLibrary.RandomPointInBoundingBox` _origin _boxextent)) "Undefined" "OverrideRootScale" null null))
    (set `/Game/Blueprints/BP_RescourceNode.Resource Multiplier` (`self.Resource Multipler`) _returnvalue)
    (set `/Game/Blueprints/BP_RescourceNode.ResourceAmount` (`self.Resource Amount`) _returnvalue)
    (set `/Game/Blueprints/BP_RescourceNode.SpawnTime` 30.0 _returnvalue)))

(fn `GenerateNodes`)

(fn `SpawnNewNode`
  (params (MinX :type "Float (double-precision)") (MaxX :type "Float (double-precision)") (MinZ :type "Float (double-precision)") (MaxZ :type "Float (double-precision)") (NodeArray :type "Array of /Game/Blueprints/BP_RescourceNode Object Reference") (RescourceMultiplier :type Integer))
  (bind _returnvalue (`KismetMathLibrary.MakeVector` 0.0))
  (bind _returnvalue_2 (`KismetMathLibrary.RandomPointInBoundingBox` _returnvalue (`KismetMathLibrary.MakeVector` MaxX MaxZ)))
  (while (`KismetMathLibrary.IsPointInBox` _returnvalue_2 _returnvalue (`KismetMathLibrary.MakeVector` MinX MinZ))
    _)
  (bind _returnvalue_3 (`|SpawnActorFromClass` "/Game/Blueprints/BP_RescourceNode.BP_RescourceNode_C" (`KismetMathLibrary.MakeTransform` _returnvalue_2) "Undefined" "OverrideRootScale" null null))
  (set `/Game/Blueprints/BP_RescourceNode.ResourceAmount` (`local.RescourceMultiplier`) _returnvalue_3)
  (set `/Game/Blueprints/BP_RescourceNode.SpawnTime` 150.0 _returnvalue_3)
  (`KismetArrayLibrary.Array_Add` (`local.NodeArray`) _returnvalue_3))

(fn `UserConstructionScript`)