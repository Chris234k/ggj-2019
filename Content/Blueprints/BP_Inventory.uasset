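; Inventory Blueprint that tracks Oxygen, Power, Food and Water totals and shows them in an on-screen widget.
; On BeginPlay it creates WBP_Inventory, stores it as UI and adds it to the viewport.
; Number keys 1 to 4 each add one unit of a resource through AddResource.
; AddResource switches on the resource type and returns the new total, which the key event writes directly to the matching widget variable.
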(event `Key|One`
  (params (Key :type "Key Structure"))
  (:`Pressed`
    (bind _total (`self.AddResource` "NewEnumerator0" 1))
    (set `/Game/Blueprints/WBP_Inventory.Oxygen` _total (`self.UI`))))

(event `Key|Two`
  (params (Key :type "Key Structure"))
  (:`Pressed`
    (bind _total (`self.AddResource` "NewEnumerator1" 1))
    (set `/Game/Blueprints/WBP_Inventory.Power` _total (`self.UI`))))

(event `Key|Three`
  (params (Key :type "Key Structure"))
  (:`Pressed`
    (bind _total (`self.AddResource` "NewEnumerator2" 1))
    (set `/Game/Blueprints/WBP_Inventory.Food` _total (`self.UI`))))

(event `Key|Four`
  (params (Key :type "Key Structure"))
  (:`Pressed`
    (bind _total (`self.AddResource` "NewEnumerator3" 1))
    (set `/Game/Blueprints/WBP_Inventory.Water` _total (`self.UI`))))

(event `self.ReceiveBeginPlay`
  (bind _returnvalue (`|CreateWidget` "/Game/Blueprints/WBP_Inventory.WBP_Inventory_C"))
  (bind _output_get (set `self.UI` _returnvalue))
  (`UserWidget.AddToViewport` _output_get 0))

(fn `AddResource`
  (params (resource :type "/Game/Blueprints/EResourceType Enum" :default "NewEnumerator0") (amount :type Integer))
  (returns (total :type Integer))
  (switch `/Game/Blueprints/EResourceType` resource
    (:`NewEnumerator0`
      (bind _output_get (set `self.Oxygen` (+ amount (`self.Oxygen`))))
      (return _output_get))
    (:`NewEnumerator1`
      (bind _output_get_2 (set `self.Power` (+ amount (`self.Power`))))
      (return _output_get_2))
    (:`NewEnumerator2`
      (bind _output_get_3 (set `self.Food` (+ amount (`self.Food`))))
      (return _output_get_3))
    (:`NewEnumerator3`
      (bind _output_get_4 (set `self.Water` (+ amount (`self.Water`))))
      (return _output_get_4))))

(fn `UserConstructionScript`)