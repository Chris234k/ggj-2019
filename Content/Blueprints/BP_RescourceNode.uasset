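; Resource node actor that spawns a BP_Power item at its own transform on BeginPlay and respawns it after a SpawnTime delay whenever Renew is called.
; Spawning only happens when CurrentItem is invalid, so the node tracks one item at a time.
; Each item gets random Power around ResourceMultiplier times ResourceAmount.
; Selection by RescourceType from ItemsToSpawn and Oxygen, Food and Water assignments are present but unused.
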(event `self.ReceiveBeginPlay`
  (`self.AttemptToSpawn` :!label _label))

(event `Event Renew`
  (`KismetSystemLibrary.Delay` (`self.SpawnTime`))
  (goto _label))

(fn `AttemptToSpawn`
  (`/Engine/EditorBlueprintResources/StandardMacros.IsValid` (`self.CurrentItem`)
    (:`Is Not Valid`
      (`self.SpawnItem`))))

(fn `SpawnItem`
  (bind _returnvalue (* (`self.Resource Multiplier`) (`self.ResourceAmount`)))
  (bind _returnvalue_2 (`|SpawnActorFromClass` "/Game/Blueprints/RescourceTypes/BP_Power.BP_Power_C" (`KismetMathLibrary.MakeTransform` (`self.K2_GetActorLocation`) (`self.K2_GetActorRotation`)) "AdjustIfPossibleButAlwaysSpawn" "OverrideRootScale" self null))
  (set `/Game/Blueprints/BP_Item.Power` (`KismetMathLibrary.RandomIntegerInRange` (`KismetMathLibrary.Max` 1 (- _returnvalue 5)) (+ _returnvalue 5)) _returnvalue_2)
  (set `self.CurrentItem` _returnvalue_2))

(fn `UserConstructionScript`)